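; Enemy pawn blueprint that chases and damages the player's BP_testCharacter and can be killed.
; PawnSensing sight triggers AI MoveTo toward the player, and a Box overlap applies a large flat hit of damage.
; Incoming damage lowers Health and pushes it to an enemyHealth widget cached on BeginPlay.
; When Health drops below zero it sets IsDead and destroys itself after a short delay.
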(event OnComponentBeginOverlap(Box)
  (params (OverlappedComponent :type Primitive%20Component%20Object%20Reference) (OtherActor :type Actor%20Object%20Reference) (OtherComp :type Primitive%20Component%20Object%20Reference) (OtherBodyIndex :type Integer) (bFromSweep :type Boolean) (SweepResult :type Hit%20Result%20Structure%20%28by%20ref%29))
  ;[1 1 1] Apply Damage
  (bind _asbp_test_character (Utilities|Casting|CastToBP_testCharacter OtherActor))
  (Game|Damage|ApplyDamage _asbp_test_character 1e+02 0 0))

(event OnSeePawn(PawnSensing)
  (params (Pawn :type Pawn%20Object%20Reference))
  ;[1 1 1] Follow
  (bind _asbp_test_character (Utilities|Casting|CastToBP_testCharacter Pawn))
  (AI|AIMoveTo self "0, 0, 0" _asbp_test_character 5.0 false))

(event Game|Damage|EventAnyDamage
  (params (Damage :type Float%20%28single-precision%29) (DamageType :type Damage%20Type%20Object%20Reference) (InstigatedBy :type Controller%20Object%20Reference) (DamageCauser :type Actor%20Object%20Reference))
  ;[1 1 1] Receive Damage
  (bind _output_get (Variables|Default|SetHealth (- (Variables|Default|GetHealth) Damage)))
  (Variables|/Game/Blueprints/enemyHealth.enemyHealth_C|SetAIHealth (Variables|Default|GetHealthWidgetRef) _output_get)
  (if (< (Variables|Default|GetHealth) 0.0)
    (Variables|Default|SetIsDead? true)
    (Utilities|FlowControl|Delay 0.2)
    (Actor|DestroyActor)))

(event EventBeginPlay
  ;[1 1 1] Link to widget
  (bind _asenemy_health (Utilities|Casting|CastToenemyHealth (UserInterface|GetUserWidgetObject (Variables|Default|GetWidget))))
  (bind _output_get (Variables|Default|SetHealthWidgetRef _asenemy_health)))

(fn ConstructionScript)