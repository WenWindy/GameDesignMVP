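; BP_Client is an interactable client that ends the game with a rating based on the evidence the player has collected.
; Its box overlap shows and removes an interact prompt for the player character.
; Interact fires Conversation, which queries the player's inventory for five clue items and counts those found.
; The count selects one of three star-system widgets for all, most or few clues, then the game quits after a short delay.
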(event OnComponentBeginOverlap(Box)
  (params (OverlappedComponent :type Primitive%20Component%20Object%20Reference) (OtherActor :type Actor%20Object%20Reference) (OtherComp :type Primitive%20Component%20Object%20Reference) (OtherBodyIndex :type Integer) (bFromSweep :type Boolean) (SweepResult :type Hit%20Result%20Structure%20%28by%20ref%29))
  (Utilities|Casting|CastToBP_testCharacter OtherActor)
  (bind _returnvalue (UserInterface|CreateWidget "/Game/Blueprints/Interact_Prompt_Widget.Interact_Prompt_Widget_C"))
  (UserInterface|Viewport|AddtoViewport _returnvalue 0))

(event OnComponentEndOverlap(Box)
  (params (OverlappedComponent :type Primitive%20Component%20Object%20Reference) (OtherActor :type Actor%20Object%20Reference) (OtherComp :type Primitive%20Component%20Object%20Reference) (OtherBodyIndex :type Integer))
  (Utilities|Casting|CastToBP_testCharacter OtherActor)
  (Widget|RemovefromParent (stale OnComponentBeginOverlap(Box) _returnvalue)))

(event Custom|Conversation
  ;[1 1 1] Inventory Query +Win Condition
  (bind _asbp_test_character (Utilities|Casting|CastToBP_testCharacter (Game|GetPlayerCharacter 0)))
  (bind _isininventory (Default|InventoryQuery (Variables|/Game/BP_testCharacter.BP_testCharacter_C|GetInventoryComponent _asbp_test_character) "/Game/InventorySystem/Item/Item_Photo.Item_Photo_C" 1))
  (if _isininventory
    (Variables|Default|SetCollectedItemNum (+ (Variables|Default|GetCollectedItemNum) 1)))
  (bind _isininventory_2 (Default|InventoryQuery (Variables|/Game/BP_testCharacter.BP_testCharacter_C|GetInventoryComponent _asbp_test_character) "/Game/InventorySystem/Item/Item_Notebook.Item_Notebook_C" 1))
  (if _isininventory_2
    (Variables|Default|SetCollectedItemNum (+ (Variables|Default|GetCollectedItemNum) 1)))
  (bind _isininventory_3 (Default|InventoryQuery (Variables|/Game/BP_testCharacter.BP_testCharacter_C|GetInventoryComponent _asbp_test_character) "/Game/InventorySystem/Item/Item_Wound.Item_Wound_C" 1))
  (if _isininventory_3
    (Variables|Default|SetCollectedItemNum (+ (Variables|Default|GetCollectedItemNum) 1)))
  (bind _isininventory_4 (Default|InventoryQuery (Variables|/Game/BP_testCharacter.BP_testCharacter_C|GetInventoryComponent _asbp_test_character) "/Game/InventorySystem/Item/Item_Fingerprint.Item_Fingerprint_C" 1))
  (if _isininventory_4
    (Variables|Default|SetCollectedItemNum (+ (Variables|Default|GetCollectedItemNum) 1)))
  (bind _isininventory_5 (Default|InventoryQuery (Variables|/Game/BP_testCharacter.BP_testCharacter_C|GetInventoryComponent _asbp_test_character) "/Game/InventorySystem/Item/Item_Bloodstain.Item_Bloodstain_C" 1))
  (if _isininventory_5
    (bind _output_get (Variables|Default|SetCollectedItemNum (+ (Variables|Default|GetCollectedItemNum) 1))))
  (if (== _output_get 5)
    (bind _returnvalue (UserInterface|CreateWidget "/Game/Blueprints/StarSystem.StarSystem_C"))
    (UserInterface|Viewport|AddtoViewport _returnvalue 0)
    (Utilities|FlowControl|Delay 5.0)
    (Game|QuitGame 0 "Quit" false)
    (elif (and (>= _output_get 3) (< _output_get 5))
      (bind _returnvalue_2 (UserInterface|CreateWidget "/Game/Blueprints/StarSystem1.StarSystem1_C"))
      (UserInterface|Viewport|AddtoViewport _returnvalue_2 0)
      (Utilities|FlowControl|Delay 5.0)
      (Game|QuitGame 0 "Quit" false)
      (else
        (bind _returnvalue_3 (UserInterface|CreateWidget "/Game/Blueprints/StarSystem2.StarSystem2_C"))
        (UserInterface|Viewport|AddtoViewport _returnvalue_3 0)
        (Utilities|FlowControl|Delay 5.0)
        (Game|QuitGame 0 "Quit" false)))))

(fn ConstructionScript)

(fn Interact
  (params (Interacter :type Actor%20Object%20Reference))
  (CallFunction|Conversation)
  (return true))