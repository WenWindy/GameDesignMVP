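; BP_EnemySpawner is an actor that spawns a limited series of BP_Enemies AI pawns at its own location, then destroys itself.
; Tick feeds a Delay with a random duration of up to fifteen seconds, so the latent node paces a repeating spawn loop without a timer.
; Each spawn increments RoundCount, and the actor is destroyed once the count reaches five.
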(event EventTick
  (params (DeltaSeconds :type Float%20%28single-precision%29))
  (Utilities|FlowControl|Delay (Math|Random|RandomFloatinRange 0.0 15.0))
  (AI|SpawnAIFromClass "/Game/BP_Enemies.BP_Enemies_C" 0 (Transformation|GetWorldLocation (Variables|Default|GetDefaultSceneRoot)) "0, 0, 0" false 0)
  (bind _output_get (Variables|Default|SetRoundCount (+ (Variables|Default|GetRoundCount) 1)))
  (if (>= _output_get 5)
    (Actor|DestroyActor)))

(fn ConstructionScript)