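; An interactable door that swings open and loads the "Client" level.
; Interact calls OpenDoor, where a FlipFlop alternates a timeline between playing forward and reversing to yaw the Pivot.
; Each timeline update, in either direction, also feeds a half-second Delay before the level load, so closing triggers it too.
; Box overlap by BP_testCharacter shows an interact prompt widget and removes it on exit.
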(event OnComponentBeginOverlap(Box)
  (params (OverlappedComponent :type Primitive%20Component%20Object%20Reference) (OtherActor :type Actor%20Object%20Reference) (OtherComp :type Primitive%20Component%20Object%20Reference) (OtherBodyIndex :type Integer) (bFromSweep :type Boolean) (SweepResult :type Hit%20Result%20Structure%20%28by%20ref%29))
  (Utilities|Casting|CastToBP_testCharacter OtherActor)
  (bind _returnvalue (UserInterface|CreateWidget "/Game/Blueprints/Interact_Prompt_Widget.Interact_Prompt_Widget_C"))
  (UserInterface|Viewport|AddtoViewport _returnvalue 0))

(event OnComponentEndOverlap(Box)
  (params (OverlappedComponent :type Primitive%20Component%20Object%20Reference) (OtherActor :type Actor%20Object%20Reference) (OtherComp :type Primitive%20Component%20Object%20Reference) (OtherBodyIndex :type Integer))
  (Utilities|Casting|CastToBP_testCharacter OtherActor)
  (Widget|RemovefromParent (stale OnComponentBeginOverlap(Box) _returnvalue)))

(event Custom|OpenDoor
  (Utilities|FlowControl|FlipFlop
    (:A
      (bind _newtrack_0 (Timeline|Door%20Timeline PlayFromStart)
        (:Update
          (Transformation|SetRelativeRotation (Variables|Default|GetPivot) (Math|Rotator|MakeRotator 0.0 0.0 _newtrack_0) false false)
          (Utilities|FlowControl|Delay 0.5)
          (Game|OpenLevel(byName) "Client"))))
    (:B
      (Timeline|Door%20Timeline ReverseFromEnd))))

(fn ConstructionScript)

(fn Interact
  (params (Interacter :type Actor%20Object%20Reference))
  (CallFunction|OpenDoor)
  (return true))