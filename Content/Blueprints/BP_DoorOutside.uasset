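; BP_DoorOutside is an interactable exterior door that swings open or closed when the player has a key.
; Interact calls OpenDoor, which queries the player's inventory for Item_Key, then a FlipFlop plays or reverses a timeline that yaws the Pivot and sets Unlocked.
; Without the key, it briefly shows either a lockpick or door message widget, depending on the equipped item.
; Box overlaps add and remove the interact prompt.
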(event OnComponentBeginOverlap(Box)
  (params (OverlappedComponent :type Primitive%20Component%20Object%20Reference) (OtherActor :type Actor%20Object%20Reference) (OtherComp :type Primitive%20Component%20Object%20Reference) (OtherBodyIndex :type Integer) (bFromSweep :type Boolean) (SweepResult :type Hit%20Result%20Structure%20%28by%20ref%29))
  (Utilities|Casting|CastToBP_testCharacter OtherActor)
  (bind _returnvalue (UserInterface|CreateWidget "/Game/Blueprints/Interact_Prompt_Widget.Interact_Prompt_Widget_C"))
  (UserInterface|Viewport|AddtoViewport _returnvalue 0))

(event OnComponentEndOverlap(Box)
  (params (OverlappedComponent :type Primitive%20Component%20Object%20Reference) (OtherActor :type Actor%20Object%20Reference) (OtherComp :type Primitive%20Component%20Object%20Reference) (OtherBodyIndex :type Integer))
  (Utilities|Casting|CastToBP_testCharacter OtherActor)
  (Widget|RemovefromParent (stale OnComponentBeginOverlap(Box) _returnvalue)))

(event Custom|OpenDoor
  (bind _asbp_test_character (Utilities|Casting|CastToBP_testCharacter (Game|GetPlayerCharacter 0)))
  (bind _isininventory (Default|InventoryQuery (Variables|/Game/BP_testCharacter.BP_testCharacter_C|GetInventoryComponent _asbp_test_character) "/Game/InventorySystem/Item/Item_Key.Item_Key_C" 1))
  (if _isininventory
    (Utilities|FlowControl|FlipFlop
      (:A
        (bind _newtrack_0 (Timeline|Door%20Timeline PlayFromStart)
          (:Update
            (Transformation|SetRelativeRotation (Variables|Default|GetPivot) (Math|Rotator|MakeRotator 0.0 0.0 _newtrack_0) false false)
            (Variables|Default|Setunlocked? true))))
      (:B
        (Timeline|Door%20Timeline ReverseFromEnd)))
    (elif (== (Variables|/Game/BP_testCharacter.BP_testCharacter_C|GetEquipped _asbp_test_character) 2)
      (bind _returnvalue (UserInterface|CreateWidget "/Game/Blueprints/OutsideLockpick_Widget.OutsideLockpick_Widget_C"))
      (UserInterface|Viewport|AddtoViewport _returnvalue 0)
      (Utilities|FlowControl|Delay 2.0)
      (Widget|RemovefromParent _returnvalue)
      (else
        (bind _returnvalue_2 (UserInterface|CreateWidget "/Game/Blueprints/OutsideDoor_Widget.OutsideDoor_Widget_C"))
        (UserInterface|Viewport|AddtoViewport _returnvalue_2 0)
        (Utilities|FlowControl|Delay 2.0)
        (Widget|RemovefromParent _returnvalue_2)))))

(fn ConstructionScript)

(fn Interact
  (params (Interacter :type Actor%20Object%20Reference))
  (CallFunction|OpenDoor)
  (return true))