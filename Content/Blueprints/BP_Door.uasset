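; Lockable hinged door that the player unlocks by interacting while the required item (Equipped index 2) is equipped, after which it stays unlocked.
; Interact calls OpenDoor, where a FlipFlop alternates playing and reversing a timeline that swings the Pivot's yaw.
; A failed unlock opens GadgetHUD with the mouse cursor and UI-only input.
; Box overlap shows and removes an interact prompt, which the Interact input briefly flags as pressed.
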(event OnComponentBeginOverlap(Box)
  (params (OverlappedComponent :type Primitive%20Component%20Object%20Reference) (OtherActor :type Actor%20Object%20Reference) (OtherComp :type Primitive%20Component%20Object%20Reference) (OtherBodyIndex :type Integer) (bFromSweep :type Boolean) (SweepResult :type Hit%20Result%20Structure%20%28by%20ref%29))
  (Utilities|Casting|CastToThirdPersonCharacter OtherActor)
  (bind _returnvalue (UserInterface|CreateWidget "/Game/Blueprints/Interact_Prompt_Widget.Interact_Prompt_Widget_C"))
  (UserInterface|Viewport|AddtoViewport _returnvalue 0))

(event OnComponentEndOverlap(Box)
  (params (OverlappedComponent :type Primitive%20Component%20Object%20Reference) (OtherActor :type Actor%20Object%20Reference) (OtherComp :type Primitive%20Component%20Object%20Reference) (OtherBodyIndex :type Integer))
  (Utilities|Casting|CastToThirdPersonCharacter OtherActor)
  (Widget|RemovefromParent (stale OnComponentBeginOverlap(Box) _returnvalue)))

(event Custom|OpenDoor
  (bind _returnvalue (Game|GetPlayerController 0))
  (bind _asthird_person_character (Utilities|Casting|CastToThirdPersonCharacter (Game|GetPlayerCharacter 0)))
  (if (or (== (Variables|/Game/ThirdPersonBP/Blueprints/ThirdPersonCharacter.ThirdPersonCharacter_C|GetEquipped _asthird_person_character) 2) (Variables|Default|GetUnlocked?))
    (Variables|Default|SetUnlocked? true)
    (Utilities|FlowControl|FlipFlop
      (:A
        (bind _newtrack_0 (Timeline|Door%20Timeline PlayFromStart)
          (:Update
            (Transformation|SetRelativeRotation (Variables|Default|GetPivot) (Math|Rotator|MakeRotator 0.0 0.0 _newtrack_0) false false))))
      (:B
        (Timeline|Door%20Timeline ReverseFromEnd)))
    (else
      (bind _returnvalue_2 (UserInterface|CreateWidget "/Game/Blueprints/GadgetHUD.GadgetHUD_C"))
      (UserInterface|Viewport|AddtoViewport _returnvalue_2 0)
      (Variables|/Script/Engine.PlayerController|SetbShowMouseCursor _returnvalue true)
      (Input|SetInputModeUIOnly _returnvalue 0 "DoNotLock"))))

(event Input|ActionEvents|InputActionInteract
  (params (Key :type Key%20Structure))
  (:Pressed
    (Variables|/Game/Blueprints/Interact_Prompt_Widget.Interact_Prompt_Widget_C|SetIs%20Pressed (stale OnComponentBeginOverlap(Box) _returnvalue) true)
    (Utilities|FlowControl|Delay 0.2)
    (Variables|/Game/Blueprints/Interact_Prompt_Widget.Interact_Prompt_Widget_C|SetIs%20Pressed (stale OnComponentBeginOverlap(Box) _returnvalue) false)))

(fn ConstructionScript)

(fn Interact
  (params (Interacter :type Actor%20Object%20Reference))
  (CallFunction|OpenDoor)
  (return true))